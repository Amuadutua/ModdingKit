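; Base Blueprint for a mod worklight that toggles between on and off states with the Use input.
; Each toggle, and BeginPlay when already on, swaps the mesh's second material, plays the WorklightOn sound and sets the ClickableComponent's use context to the opposite action.
; Tick checks available power, but nothing follows the check, so power does not affect the state here.
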(event `self.ReceiveBeginPlay`
  (if (`self.On`)
    (`PrimitiveComponent.SetMaterial` (`self.StaticMeshComponent`) 1 (`self.OnMaterial`))
    (`GameplayStatics.PlaySoundAtLocation` "/Game/Mods/TheCodingPro/ColoredLightless/Sounds/WorklightOn.WorklightOn" (`self.K2_GetActorLocation`) (struct) 1.0 1.0 0.0 null null null)
    (`ClickableComponent.SetActiveUseContext` (`self.ClickableComponent`) "UC_TurnOff")))

(event `InputAction|Use`
  (params (Key :type "Key Structure"))
  (bind _staticmeshcomponent (`self.StaticMeshComponent`))
  (bind _clickablecomponent (`self.ClickableComponent`))
  (:`Pressed`
    (if (not (`self.On`))
      (set `self.On` true)
      (`PrimitiveComponent.SetMaterial` _staticmeshcomponent 1 (`self.OnMaterial`))
      (`GameplayStatics.PlaySoundAtLocation` "/Game/Mods/TheCodingPro/ColoredLightless/Sounds/WorklightOn.WorklightOn" (`self.K2_GetActorLocation`) (struct) 1.0 1.0 0.0 null null null)
      (`ClickableComponent.SetActiveUseContext` _clickablecomponent "UC_TurnOff")
      (else
        (set `self.On` false)
        (`PrimitiveComponent.SetMaterial` _staticmeshcomponent 1 (`self.OffMaterial`))
        (`GameplayStatics.PlaySoundAtLocation` "/Game/Mods/TheCodingPro/ColoredLightless/Sounds/WorklightOn.WorklightOn" (`self.K2_GetActorLocation`) (struct) 1.0 1.0 0.0 null null null)
        (`ClickableComponent.SetActiveUseContext` _clickablecomponent "UC_TurnOn")))))

(event `self.ReceiveTick`
  (params (DeltaSeconds :type "Float (single-precision)"))
  (if (> (`KismetMathLibrary.Abs` (`PowerComponent.CurrentAvailablePower` (`self.Power`))) 0.0)
    _))

(fn `GetBodySlotLegacy`
  (returns (ReturnValue :type "ChildSlotComponent Object Reference"))
  (return (`self.BodySlot`)))

(fn `UserConstructionScript`)