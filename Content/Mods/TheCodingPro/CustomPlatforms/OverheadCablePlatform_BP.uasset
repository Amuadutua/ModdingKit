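; OverheadCablePlatform_BP is a modded overhead cable platform that a player can lock or unlock with the Use action.
; Pressing Use toggles IsMovable, plays the matching lock or unlock sound and switches the ClickableComponent's use context to show the opposite action.
; On BeginPlay it restores the Unlock context when the platform is not movable, so the locked state carries across save reloads.
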(event `InputAction|Use`
  (params (Key :type "Key Structure"))
  (bind _clickablecomponent (`self.ClickableComponent`))
  (:`Pressed`
    (if (`self.IsMovable`)
      ;[1 1 1] Sets IsMovable to true or false
      (set `self.IsMovable` false)
      ;[1 1 1] Plays locking or unlocking sound
      (`AstroStatics.PlaySound` "/Game/Mods/TheCodingPro/CustomPlatforms/LockPlatform.LockPlatform")
      ;[1 1 1] The SetActiveUseContext method allows you to change what displays as the use action and automatically refreshes active tooltips if necessary
      (`ClickableComponent.SetActiveUseContext` _clickablecomponent "UC_Unlock")
      (else
        (set `self.IsMovable` true)
        (`AstroStatics.PlaySound` "/Game/Mods/TheCodingPro/CustomPlatforms/UnlockPlatform.UnlockPlatform")
        (`ClickableComponent.SetActiveUseContext` _clickablecomponent "UC_Lock")))))

(event `self.ReceiveBeginPlay`
  ;[1 1 1] Keeps platform locked between reloading save
  (if (not (`self.IsMovable`))
    (`ClickableComponent.SetActiveUseContext` (`self.ClickableComponent`) "UC_Unlock")))

(fn `GetBodySlotLegacy`
  (returns (ReturnValue :type "ChildSlotComponent Object Reference"))
  (return (`self.BodySlot`)))

(fn `UserConstructionScript`)