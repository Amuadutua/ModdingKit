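; Anti-grief shield from a mod, with a Use input that toggles it and swaps bubble and glow materials.
; While on, sphere overlaps clear platform lockdown on authority (despite a comment saying lock), strip the local player's terrain tool, and destroy explosive actors.
; Each such overlap also adds a bright point light.
; Nothing reverses these effects on exit or switch-off.
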(event `InputAction|Use`
  (params (Key :type "Key Structure"))
  (bind _staticmeshcomponent (`self.StaticMeshComponent`))
  (bind _bubble (`self.Bubble`))
  (:`Pressed`
    (if (not (`self.On`))
      (set `self.On` true)
      (`PrimitiveComponent.SetMaterial` _bubble 0 "/Game/Mods/TheCodingPro/AntiGriefMod/Materials/BorderActiveMat.BorderActiveMat")
      (`PrimitiveComponent.SetMaterial` _staticmeshcomponent 1 "/Game/Mods/TheCodingPro/AntiGriefMod/Materials/GlowActiveMat.GlowActiveMat")
      (else
        (set `self.On` false)
        (`PrimitiveComponent.SetMaterial` _bubble 0 "/Game/Mods/TheCodingPro/AntiGriefMod/Materials/BorderInactiveMat.BorderInactiveMat")
        (`PrimitiveComponent.SetMaterial` _staticmeshcomponent 1 "/Game/Mods/TheCodingPro/AntiGriefMod/Materials/GlowInactiveMat.GlowInactiveMat")))))

(event `self.Sphere.OnComponentBeginOverlap`
  (params (OverlappedComponent :type "PrimitiveComponent Object Reference") (OtherActor :type "Actor Object Reference") (OtherComp :type "PrimitiveComponent Object Reference") (OtherBodyIndex :type Integer) (bFromSweep :type Boolean) (SweepResult :type "HitResult Structure (by ref)"))
  (bind _returnvalue (`self.GetComponentByClass` OtherActor "/Script/Astro.BreadboardPlatformComponent"))
  (bind _returnvalue_2 (`AstroPlayStatics.GetLocalAstroCharacter`))
  (if (`self.On`)
    (`|ExecutionSequence`
      (:`then_0`
        ;[0.4794 0.8275 1] Checks if the item in the zone is a platform, and locks it if so
        (if (`KismetSystemLibrary.IsValid` _returnvalue)
          (`/Engine/EditorBlueprintResources/ActorMacros.Switch Has Authority`
            (:`Authority`
              (`BreadboardPlatformComponent.AuthoritySetLockdownEnabled` _returnvalue false)))))
      (:`then_1`
        ;[1 1 1] Removes the DeformTool when player in zone
        (if (== OtherActor _returnvalue_2)
          (set `AstroPlayerState.bAuthorityHasAcquiredTerrainTool` false (`self.Player State`))
          (`self.K2_DestroyActor` (`AstroCharacter.GetDeformTool` _returnvalue_2))))
      (:`then_2`
        ;[1 0.2851 0.2154] Checks whether the item found within the zone has an explosive component and if true then destroys it
        (if (`KismetSystemLibrary.IsValid` (`self.GetComponentByClass` OtherActor "/Script/Astro.ExplosiveComponent"))
          (`self.K2_DestroyActor` OtherActor)))
      (:`then_3`
        (bind _returnvalue_3 (`AddComponent|NODE_AddPointLightComponent-0` :`RelativeTransform` (`KismetMathLibrary.MakeTransform` (0.0 0.0 0.0))))
        (`LightComponent.SetIntensity` _returnvalue_3 10000.0)
        (`LocalLightComponent.SetAttenuationRadius` _returnvalue_3 10000.0)))))

(fn `GetBodySlotLegacy`
  (returns (ReturnValue :type "ChildSlotComponent Object Reference"))
  (return (`self.BodySlot`)))

(fn `UserConstructionScript`)