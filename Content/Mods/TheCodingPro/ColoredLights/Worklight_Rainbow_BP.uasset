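; Rainbow worklight Blueprint from the ColoredLights mod: a switchable, powered lamp that changes color.
; A timeline started on BeginPlay writes one color to both the point light and the dynamic emitter material, keeping them in sync.
; Use input toggles light, material, sound and click context.
; Tick blacks out the lamp without power; when powered and enabled, it recreates the material every frame and overrides brightness and radius with lower values.
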(event `self.ReceiveBeginPlay`
  (bind _pointlight (`self.PointLight`))
  (`|ExecutionSequence`
    (:`then_0`
      (if (`self.LightEnabled`)
        (bind _returnvalue (`PrimitiveComponent.CreateDynamicMaterialInstance` (`self.StaticMeshComponent`) 1 "/Game/Mods/TheCodingPro/ColoredLights/Materials/LightMatRainbowEnabled.LightMatRainbowEnabled" "None"))
        (set `self.Material` _returnvalue)
        (`LightComponent.SetIntensity` _pointlight 10000.0)
        (`LocalLightComponent.SetAttenuationRadius` _pointlight 5000.0)
        (`ClickableComponent.SetActiveUseContext` (`self.ClickableComponent`) "UC_TurnOff")))
    (:`then_1`
      ;[1 1 1] Timer for syncing the light and the material
      (bind (_direction _colorchange) (`Timeline|ColorTimer` :!via `PlayFromStart`)
        (:`Update`
          (`MaterialInstanceDynamic.SetVectorParameterValue` (`self.Material`) "Color" _colorchange)
          (`LightComponent.SetLightColor` (`self.PointLight`) _colorchange true))))))

(event `InputAction|Use`
  (params (Key :type "Key Structure"))
  (bind _returnvalue (`self.K2_GetActorLocation`))
  (bind _staticmeshcomponent (`self.StaticMeshComponent`))
  (bind _clickablecomponent (`self.ClickableComponent`))
  (bind _pointlight (`self.PointLight`))
  (:`Pressed`
    (if (not (`self.LightEnabled`))
      (set `self.LightEnabled` true)
      (bind _returnvalue_2 (`PrimitiveComponent.CreateDynamicMaterialInstance` _staticmeshcomponent 1 "/Game/Mods/TheCodingPro/ColoredLights/Materials/LightMatRainbowEnabled.LightMatRainbowEnabled" "None"))
      (set `self.Material` _returnvalue_2)
      (`GameplayStatics.PlaySoundAtLocation` "/Game/Mods/TheCodingPro/ColoredLights/Sounds/WorklightOn.WorklightOn" _returnvalue (struct) 1.0 1.0 0.0 null null null)
      (`LightComponent.SetIntensity` _pointlight 10000.0)
      (`LocalLightComponent.SetAttenuationRadius` _pointlight 5000.0)
      (`ClickableComponent.SetActiveUseContext` _clickablecomponent "UC_TurnOff")
      (else
        (set `self.LightEnabled` false)
        (`PrimitiveComponent.SetMaterial` _staticmeshcomponent 1 "/Game/Mods/TheCodingPro/ColoredLights/Materials/WorklightMatDisabled.WorklightMatDisabled")
        (`GameplayStatics.PlaySoundAtLocation` "/Game/Mods/TheCodingPro/ColoredLights/Sounds/WorklightOff.WorklightOff" _returnvalue (struct) 1.0 1.0 0.0 null null null)
        (`LightComponent.SetIntensity` _pointlight 0.0)
        (`LocalLightComponent.SetAttenuationRadius` _pointlight 0.0)
        (`ClickableComponent.SetActiveUseContext` _clickablecomponent "UC_TurnOn")))))

(event `self.ReceiveTick`
  (params (DeltaSeconds :type "Float (single-precision)"))
  (bind _staticmeshcomponent (`self.StaticMeshComponent`))
  (bind _pointlight (`self.PointLight`))
  (if (> (`KismetMathLibrary.Abs` (`PowerComponent.CurrentAvailablePower` (`self.Power`))) 0.0)
    (if (`self.LightEnabled`)
      (bind _returnvalue (`PrimitiveComponent.CreateDynamicMaterialInstance` _staticmeshcomponent 1 "/Game/Mods/TheCodingPro/ColoredLights/Materials/LightMatRainbowEnabled.LightMatRainbowEnabled" "None"))
      (set `self.Material` _returnvalue)
      (`LightComponent.SetIntensity` _pointlight 5000.0)
      (`LocalLightComponent.SetAttenuationRadius` _pointlight 1000.0))
    (else
      (`PrimitiveComponent.SetMaterial` _staticmeshcomponent 1 "/Game/Mods/TheCodingPro/ColoredLights/Materials/WorklightMatDisabled.WorklightMatDisabled")
      (`LightComponent.SetIntensity` _pointlight 0.0)
      (`LocalLightComponent.SetAttenuationRadius` _pointlight 0.0))))

(fn `UserConstructionScript`)