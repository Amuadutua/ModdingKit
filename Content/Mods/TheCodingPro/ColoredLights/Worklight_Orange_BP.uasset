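; Orange worklight from the ColoredLights mod: a powered light the player switches on and off with the Use input.
; Use flips LightEnabled, swapping the lamp material, point light intensity and radius, sound and clickable prompt; BeginPlay reapplies the enabled state.
; Tick polls available power, blanking the light and prompt indicators without it and relighting when power returns, since LightEnabled is preserved.
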(event `self.ReceiveBeginPlay`
  (bind _pointlight (`self.PointLight`))
  (if (`self.LightEnabled`)
    (`GameplayStatics.PlaySoundAtLocation` "/Game/Mods/TheCodingPro/ColoredLights/Sounds/WorklightOn.WorklightOn" (`self.K2_GetActorLocation`) (struct) 1.0 1.0 0.0 null null null)
    (`PrimitiveComponent.SetMaterial` (`self.StaticMeshComponent`) 1 "/Game/Mods/TheCodingPro/ColoredLights/Materials/LightMatOrangeEnabled.LightMatOrangeEnabled")
    (`LightComponent.SetIntensity` _pointlight 10000.0)
    (`LocalLightComponent.SetAttenuationRadius` _pointlight 5000.0)
    (`ClickableComponent.SetActiveUseContext` (`self.ClickableComponent`) "UC_TurnOff")))

(event `InputAction|Use`
  (params (Key :type "Key Structure"))
  (bind _returnvalue (`self.K2_GetActorLocation`))
  (bind _staticmeshcomponent (`self.StaticMeshComponent`))
  (bind _pointlight (`self.PointLight`))
  (bind _clickablecomponent (`self.ClickableComponent`))
  (:`Pressed`
    (if (not (`self.LightEnabled`))
      (set `self.LightEnabled` true)
      (`PrimitiveComponent.SetMaterial` _staticmeshcomponent 1 "/Game/Mods/TheCodingPro/ColoredLights/Materials/LightMatOrangeEnabled.LightMatOrangeEnabled")
      (`GameplayStatics.PlaySoundAtLocation` "/Game/Mods/TheCodingPro/ColoredLights/Sounds/WorklightOn.WorklightOn" _returnvalue (struct) 1.0 1.0 0.0 null null null)
      (`LightComponent.SetIntensity` _pointlight 10000.0)
      (`LocalLightComponent.SetAttenuationRadius` _pointlight 5000.0)
      (`ClickableComponent.SetActiveUseContext` _clickablecomponent "UC_TurnOff")
      (else
        (set `self.LightEnabled` false)
        (`PrimitiveComponent.SetMaterial` _staticmeshcomponent 1 "/Game/Mods/TheCodingPro/ColoredLights/Materials/WorklightMatDisabled.WorklightMatDisabled")
        (`GameplayStatics.PlaySoundAtLocation` "/Game/Mods/TheCodingPro/ColoredLights/Sounds/WorklightOff.WorklightOff" _returnvalue (struct) 1.0 1.0 0.0 null null null)
        (`LightComponent.SetIntensity` _pointlight 0.0)
        (`LocalLightComponent.SetAttenuationRadius` _pointlight 0.0)
        (`ClickableComponent.SetActiveUseContext` _clickablecomponent "UC_TurnOn")))))

(event `self.ReceiveTick`
  (params (DeltaSeconds :type "Float (single-precision)"))
  (bind _pointlight (`self.PointLight`))
  (bind _pointlight_2 (`self.PointLight`))
  (bind _clickablecomponent (`self.ClickableComponent`))
  (if (> (`KismetMathLibrary.Abs` (`PowerComponent.CurrentAvailablePower` (`self.Power`))) 0.0)
    (set `ClickableComponent.ShowPrimaryIndicator` true _clickablecomponent)
    (set `ClickableComponent.ShowPrimaryIcon` true _clickablecomponent)
    (if (`self.LightEnabled`)
      (`PrimitiveComponent.SetMaterial` (`self.StaticMeshComponent`) 1 "/Game/Mods/TheCodingPro/ColoredLights/Materials/LightMatOrangeEnabled.LightMatOrangeEnabled")
      (`LightComponent.SetIntensity` _pointlight 10000.0)
      (`LocalLightComponent.SetAttenuationRadius` _pointlight 5000.0))
    (else
      (set `ClickableComponent.ShowPrimaryIndicator` false _clickablecomponent)
      (set `ClickableComponent.ShowPrimaryIcon` false _clickablecomponent)
      (`PrimitiveComponent.SetMaterial` (`self.StaticMeshComponent`) 1 "/Game/Mods/TheCodingPro/ColoredLights/Materials/WorklightMatDisabled.WorklightMatDisabled")
      (`LightComponent.SetIntensity` _pointlight_2 0.0)
      (`LocalLightComponent.SetAttenuationRadius` _pointlight_2 0.0))))

(fn `UserConstructionScript`
  (`parent.UserConstructionScript`))