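; Purple floodlight from the ColoredLights mod, a powered light that the player toggles with the Use action.
; Toggling flips LightEnabled, swapping two mesh materials, spotlight intensity and radius, the use prompt, and playing an on or off sound.
; BeginPlay applies the lit state and sound if already enabled.
; Tick polls available power every frame, forcing the light dark without power and reapplying the lit look when powered and enabled.
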(event `self.ReceiveBeginPlay`
  (bind _spotlight (`self.SpotLight`))
  (bind _staticmeshcomponent (`self.StaticMeshComponent`))
  (if (`self.Light Enabled`)
    (`GameplayStatics.PlaySoundAtLocation` "/Game/Mods/TheCodingPro/ColoredLights/Sounds/WorklightOn.WorklightOn" (`self.K2_GetActorLocation`) (struct) 1.0 1.0 0.0 null null null)
    (`PrimitiveComponent.SetMaterial` _staticmeshcomponent 1 "/Game/Mods/TheCodingPro/ColoredLights/Materials/LightMatPurpleEnabled.LightMatPurpleEnabled")
    (`PrimitiveComponent.SetMaterial` _staticmeshcomponent 2 "/Game/Mods/TheCodingPro/ColoredLights/Materials/LightMatPurpleEnabled.LightMatPurpleEnabled")
    (`LightComponent.SetIntensity` _spotlight 250000.0)
    (`LocalLightComponent.SetAttenuationRadius` _spotlight 150000.0)
    (`ClickableComponent.SetActiveUseContext` (`self.ClickableComponent`) "UC_TurnOff")))

(event `InputAction|Use`
  (params (Key :type "Key Structure"))
  (bind _returnvalue (`self.K2_GetActorLocation`))
  (bind _clickablecomponent (`self.ClickableComponent`))
  (bind _spotlight (`self.SpotLight`))
  (bind _staticmeshcomponent (`self.StaticMeshComponent`))
  (:`Pressed`
    (if (not (`self.Light Enabled`))
      (set `self.Light Enabled` true)
      (`PrimitiveComponent.SetMaterial` _staticmeshcomponent 1 "/Game/Mods/TheCodingPro/ColoredLights/Materials/LightMatPurpleEnabled.LightMatPurpleEnabled")
      (`PrimitiveComponent.SetMaterial` _staticmeshcomponent 2 "/Game/Mods/TheCodingPro/ColoredLights/Materials/LightMatPurpleEnabled.LightMatPurpleEnabled")
      (`GameplayStatics.PlaySoundAtLocation` "/Game/Mods/TheCodingPro/ColoredLights/Sounds/WorklightOn.WorklightOn" _returnvalue (struct) 1.0 1.0 0.0 null null null)
      (`LightComponent.SetIntensity` _spotlight 250000.0)
      (`LocalLightComponent.SetAttenuationRadius` _spotlight 150000.0)
      (`ClickableComponent.SetActiveUseContext` _clickablecomponent "UC_TurnOff")
      (else
        (set `self.Light Enabled` false)
        (`PrimitiveComponent.SetMaterial` _staticmeshcomponent 1 "/Game/Mods/TheCodingPro/ColoredLights/Materials/FloodlightOuterCone_Base.FloodlightOuterCone_Base")
        (`PrimitiveComponent.SetMaterial` _staticmeshcomponent 2 "/Game/Mods/TheCodingPro/ColoredLights/Materials/FloodlightGlow_Base.FloodlightGlow_Base")
        (`GameplayStatics.PlaySoundAtLocation` "/Game/Mods/TheCodingPro/ColoredLights/Sounds/WorklightOff.WorklightOff" _returnvalue (struct) 1.0 1.0 0.0 null null null)
        (`LightComponent.SetIntensity` _spotlight 0.0)
        (`LocalLightComponent.SetAttenuationRadius` _spotlight 0.0)
        (`ClickableComponent.SetActiveUseContext` _clickablecomponent "UC_TurnOn")))))

(event `self.ReceiveTick`
  (params (DeltaSeconds :type "Float (single-precision)"))
  (bind _spotlight (`self.SpotLight`))
  (bind _staticmeshcomponent (`self.StaticMeshComponent`))
  (if (> (`PowerComponent.CurrentAvailablePower` (`self.Power`)) 0.0)
    (if (`self.Light Enabled`)
      (`PrimitiveComponent.SetMaterial` _staticmeshcomponent 1 "/Game/Mods/TheCodingPro/ColoredLights/Materials/LightMatPurpleEnabled.LightMatPurpleEnabled")
      (`PrimitiveComponent.SetMaterial` _staticmeshcomponent 2 "/Game/Mods/TheCodingPro/ColoredLights/Materials/LightMatPurpleEnabled.LightMatPurpleEnabled")
      (`LightComponent.SetIntensity` _spotlight 250000.0)
      (`LocalLightComponent.SetAttenuationRadius` _spotlight 150000.0))
    (else
      (`PrimitiveComponent.SetMaterial` _staticmeshcomponent 1 "/Game/Mods/TheCodingPro/ColoredLights/Materials/FloodlightOuterCone_Base.FloodlightOuterCone_Base")
      (`PrimitiveComponent.SetMaterial` _staticmeshcomponent 2 "/Game/Mods/TheCodingPro/ColoredLights/Materials/FloodlightGlow_Base.FloodlightGlow_Base")
      (`LightComponent.SetIntensity` _spotlight 0.0)
      (`LocalLightComponent.SetAttenuationRadius` _spotlight 0.0))))

(fn `UserConstructionScript`
  (`parent.UserConstructionScript`))