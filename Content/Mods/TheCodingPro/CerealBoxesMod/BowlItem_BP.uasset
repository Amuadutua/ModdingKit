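; Bowl item for the CerealBoxes mod that consumes items placed in its slots and drives a Fruity Pebbles timer.
; Placing an item calls the timer's OnInvincibilityStarted, then destroys that slot's item; the ReleasedfromSlot event calls the timer's EndEvent.
; A class check for the Fruity Pebbles item is disconnected, so placement is not filtered by item type.
; GetBodySlotLegacy returns the attachment slot.
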(event `OnItemPlacedInSlot`
  (params (Slot :type "SlotReference Structure"))
  (`/Game/Mods/TheCodingPro/CerealBoxesMod/FruityPebblesTimer.OnInvincibilityStarted` (`self.FruityPebblesTimer`))
  (`SlotsComponent.DestroySlotItem` Slot))

(event `self.ReleasedFromSlot`
  (params (FromTool :type Boolean) (NewOwner :type Boolean))
  (if true
    (`/Game/Mods/TheCodingPro/CerealBoxesMod/FruityPebblesTimer.EndEvent` (`self.FruityPebblesTimer`))))

(fn `GetBodySlotLegacy`
  (returns (ReturnValue :type "ChildSlotComponent Object Reference"))
  (return (`self.AttachmentSlot`)))

(fn `UserConstructionScript`)