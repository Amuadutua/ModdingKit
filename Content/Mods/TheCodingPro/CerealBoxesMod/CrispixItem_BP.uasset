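; Crispix cereal box item from a mod that acts as a toggle for a supercharged terrain deform tool.
; Pressing Use checks the local player's deform tool brush scale to pick between boosted and lower preset values for brush size, indicator, intensity, tier and range.
; Each branch also switches the clickable component's use context between TurnOn and TurnOff.
; No separate state is stored, as the tool's current scale serves as the toggle.
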(event `InputAction|Use`
  (params (Key :type "Key Structure"))
  (bind _clickablecomponent (`self.ClickableComponent`))
  (bind _returnvalue (`AstroCharacter.GetDeformTool` (`PlayController.GetAstroCharacter` (`AstroPlayStatics.GetLocalPlayController` self))))
  (:`Pressed`
    (if (> (`DeformTool.BaseBrushDeformationScale` _returnvalue) 400.0)
      (bind _output_get (set `DeformTool.BaseBrushDeformationScale` 350.0 _returnvalue))
      (set `DeformTool.BaseBrushIndicatorScale` _output_get _returnvalue)
      (bind _output_get_2 (set `DeformTool.BaseDeformationItensity` 1.0 _returnvalue))
      (set `DeformTool.DeformTier` _output_get_2 _returnvalue)
      (set `DeformTool.ToolRange` 1300.0 _returnvalue)
      (`ClickableComponent.SetActiveUseContext` _clickablecomponent "UC_TurnOn")
      (else
        (bind _output_get_3 (set `DeformTool.BaseBrushDeformationScale` 5000.0 _returnvalue))
        (set `DeformTool.BaseBrushIndicatorScale` _output_get_3 _returnvalue)
        (bind _output_get_4 (set `DeformTool.BaseDeformationItensity` 5000.0 _returnvalue))
        (set `DeformTool.DeformTier` _output_get_4 _returnvalue)
        (set `DeformTool.ToolRange` 100000.0 _returnvalue)
        (`ClickableComponent.SetActiveUseContext` _clickablecomponent "UC_TurnOff")))))

(fn `GetBodySlotLegacy`
  (returns (ReturnValue :type "ChildSlotComponent Object Reference"))
  (return (`self.ChildSlot`)))

(fn `UserConstructionScript`)