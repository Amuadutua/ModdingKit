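; FruityPebblesItem_BP is a cereal item from the CerealBoxes mod, Fruity Pebbles, that reacts when placed in a slot.
; On placement, if the local player's character is not invincible and the slot's owner is a BowlItem_BP, it forwards the slot to the bowl's OnItemPlacedInSlot.
; It also exposes ChildSlot as its legacy body slot.
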(event `self.PlacedInSlot`
  (params (Slot :type "SlotReference Structure") (FromTool :type Boolean) (SlottedDuringInitialization :type Boolean))
  (if (and (not (`AstroCharacter.bInvincible` (`PlayController.GetAstroCharacter` (`AstroPlayStatics.GetLocalPlayController` self)))) (== (`GameplayStatics.GetObjectClass` (`ActorComponent.GetOwner` (`SlotsComponent.GetSlotOwner` Slot))) "/Game/Mods/TheCodingPro/CerealBoxesMod/BowlItem_BP.BowlItem_BP_C"))
    (`/Game/Mods/TheCodingPro/CerealBoxesMod/BowlItem_BP.OnItemPlacedInSlot` (`self.BowlItem`) Slot)))

(fn `GetBodySlotLegacy`
  (returns (ReturnValue :type "ChildSlotComponent Object Reference"))
  (return (`self.ChildSlot`)))

(fn `UserConstructionScript`)