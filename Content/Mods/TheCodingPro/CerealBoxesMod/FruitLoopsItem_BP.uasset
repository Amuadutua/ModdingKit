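; Fruit Loops cereal box item from the CerealBoxesMod that switches the local player's gravity between two strengths.
; BeginPlay caches an AstroCharacterMovementComponent reference from the local player controller's AstroCharacter.
; The Use input action flips that component's Gravity between low and higher values, updating the ClickableComponent's TurnOn or TurnOff use context to match.
; GetBodySlotLegacy exposes ChildSlot as the body slot.
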(event `self.ReceiveBeginPlay`
  (bind _returnvalue (`AddComponent|NODE_AddAstroCharacterMovementComponent-1` :`self` (`PlayController.GetAstroCharacter` (`AstroPlayStatics.GetLocalPlayController` self)))))

(event `InputAction|Use`
  (params (Key :type "Key Structure"))
  (bind _clickablecomponent (`self.ClickableComponent`))
  (:`Pressed`
    (if (< (`AstroCharacterMovementComponent.Gravity` (stale `self.ReceiveBeginPlay` _returnvalue)) 6.5)
      (set `AstroCharacterMovementComponent.Gravity` 6.5 (stale `self.ReceiveBeginPlay` _returnvalue))
      (`ClickableComponent.SetActiveUseContext` _clickablecomponent "UC_TurnOn")
      (else
        (set `AstroCharacterMovementComponent.Gravity` 1.0 (stale `self.ReceiveBeginPlay` _returnvalue))
        (`ClickableComponent.SetActiveUseContext` _clickablecomponent "UC_TurnOff")))))

(fn `GetBodySlotLegacy`
  (returns (ReturnValue :type "ChildSlotComponent Object Reference"))
  (return (`self.ChildSlot`)))

(fn `UserConstructionScript`)