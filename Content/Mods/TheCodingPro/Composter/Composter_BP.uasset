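; Composter machine (TheCodingPro mod) that turns Organic items into Sediment while powered.
; Each Tick, if the resource slot holds Organic and the output slot's canister is not full, it adds Sediment and drains the Organic at fixed rates.
; BeginPlay caches both slot references and the storage chassis whitelist rules.
; Six debug text fields refresh every Tick with slot validity, power, canister fullness and amounts.
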(event `self.ReceiveBeginPlay`
  (bind _storagechassis (`self.StorageChassis`))
  (set `self.ResSlotRef` (`ChildSlotComponent.MakeReference` (`self.ResourceSlot`)))
  (set `self.OutSlotRef` (`ChildSlotComponent.MakeReference` (`self.OutputSlot`)))
  (bind _aswhitelist_organization_rule (cast `WhitelistOrganizationRule` (`StorageChassisComponent.FindRuleByName` _storagechassis "OutRule")))
  (set `self.InputSlotRule` _aswhitelist_organization_rule)
  (bind _aswhitelist_organization_rule_2 (cast `WhitelistOrganizationRule` (`StorageChassisComponent.FindRuleByName` _storagechassis "InputRule")))
  (set `self.OutputSlotRule` _aswhitelist_organization_rule_2))

(event `self.ReceiveTick`
  (params (DeltaSeconds :type "Float (single-precision)"))
  (bind _resslotref (`self.ResSlotRef`))
  (bind _outslotref (`self.OutSlotRef`))
  (`self.ChangeText`)
  (if (`self.CheckSlotItemValidity` _resslotref)
    (if (`self.GetPowerAvailable`)
      (bind _itemtype (`self.GetItemTypeFromPhysicalItem`))
      (if (== _itemtype "/Game/Items/ItemTypes/Minables/Organic.Organic_C")
        (if (`self.CheckSlotItemValidity` _outslotref)
          (if (not (`self.IsCanisterFull` _outslotref))
            (`ItemComponent.AddItemRateDelta` (`self.GetSlotItemComponent` _outslotref) "/Game/Items/ItemTypes/Minables/Sediment.Sediment_C" 0.005 1.0)
            (`ItemComponent.TakeItemRateDelta` (`self.GetSlotItemComponent` _resslotref) 0.02 1.0)
            (set `self.IsConsumingOrganic` true)))))))

(fn `ChangeText`
  (bind _outslotref (`self.OutSlotRef`))
  (bind _resslotref (`self.ResSlotRef`))
  (`TextRenderComponent.K2_SetText` (`self.Debuginfo_1`) (`KismetTextLibrary.Conv_StringToText` (`KismetStringLibrary.Concat_StrStr` "Organic Slot Valid: " (`KismetTextLibrary.Conv_TextToString` (`KismetTextLibrary.Conv_BoolToText` (`self.CheckSlotItemValidity` _resslotref))))))
  (`TextRenderComponent.K2_SetText` (`self.Debuginfo_2`) (`KismetTextLibrary.Conv_StringToText` (`KismetStringLibrary.Concat_StrStr` "Canister Slot Valid: " (`KismetTextLibrary.Conv_TextToString` (`KismetTextLibrary.Conv_BoolToText` (`self.CheckSlotItemValidity` _outslotref))))))
  (`TextRenderComponent.K2_SetText` (`self.Debuginfo_3`) (`KismetTextLibrary.Conv_StringToText` (`KismetStringLibrary.Concat_StrStr` "Is Powered: " (`KismetTextLibrary.Conv_TextToString` (`KismetTextLibrary.Conv_BoolToText` (`PowerComponent.IsPowered` (`self.Power`)))))))
  (`TextRenderComponent.K2_SetText` (`self.Debuginfo_4`) (`KismetTextLibrary.Conv_StringToText` (`KismetStringLibrary.Concat_StrStr` "Is Canister Full: " (`KismetTextLibrary.Conv_TextToString` (`KismetTextLibrary.Conv_BoolToText` (`self.IsCanisterFull` _outslotref))))))
  (`TextRenderComponent.K2_SetText` (`self.Debuginfo_5`) (`KismetTextLibrary.Conv_StringToText` (`KismetStringLibrary.Concat_StrStr` "Canister Soil Amount: " (`KismetStringLibrary.Conv_IntToString` (`ItemComponent.GetAmount` (`self.GetSlotItemComponent` _outslotref))))))
  (`TextRenderComponent.K2_SetText` (`self.Debuginfo_6`) (`KismetTextLibrary.Conv_StringToText` (`KismetStringLibrary.Concat_StrStr` "Organic Amount: " (`KismetStringLibrary.Conv_IntToString` (`ItemComponent.GetAmount` (`self.GetSlotItemComponent` _resslotref)))))))

(fn `GetBodySlotLegacy`
  (returns (ReturnValue :type "ChildSlotComponent Object Reference"))
  (return (`self.BodySlot`)))

(fn `GetItemTypeFromPhysicalItem`
  (returns (ItemType :type "ItemType Class Reference"))
  (return (`ItemComponent.ItemType` (`self.GetComponentByClass` (`SlotsComponent.GetSlotItem` (`self.ResSlotRef`)) "/Script/Astro.ItemComponent"))))

(fn `GetValidFuels`
  (returns (`Valid Fuels` :type "Array of Actor Class Reference"))
  (for _array_element (defaults `/Game/Mods/TheCodingPro/Composter/Composter_BP` (`WhitelistOrganizationRule.ItemTypeWhitelist` (`self.InputSlotRule`)))
    (`KismetArrayLibrary.Array_Add` (`self.Valid Fuels`) (`.PickupActor` (defaults `/Game/Mods/TheCodingPro/Composter/Composter_BP` _array_element))))
  (return (`self.Valid Fuels`)))

(fn `IsSlotItemLessThan`
  (params (Slot :type "SlotReference Structure") (CompareAmount :type Integer :default 0))
  (if (<= (`ItemComponent.GetAmount` (`self.GetSlotItemComponent` Slot)) CompareAmount)
    (if (`ItemComponent.IsFull` (`self.GetSlotItemComponent` (`self.OutSlotRef`)))
      (`SlotsComponent.DestroySlotItem` Slot))))

(fn `UserConstructionScript`)