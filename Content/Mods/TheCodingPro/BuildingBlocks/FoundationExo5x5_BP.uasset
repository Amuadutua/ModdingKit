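; FoundationExo5x5_BP is a placeable foundation building block from TheCodingPro's BuildingBlocks mod.
; On begin play, world start or slot placement, it enables mesh collision that blocks pawns.
; Dropping on terrain and pickup play lock and unlock sounds.
; Use sets StorageChassis active state and the TurnOn/TurnOff context from the Enabled flag, but each branch rewrites that flag unchanged, so it never toggles.
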(event `self.ReceiveBeginPlay`
  (bind _staticmeshcomponent (`self.StaticMeshComponent`))
  (`|ExecutionSequence`
    (:`then_0`
      (`PrimitiveComponent.SetCollisionEnabled` _staticmeshcomponent "QueryAndPhysics" :!label _label)
      (`PrimitiveComponent.SetCollisionResponseToChannel` _staticmeshcomponent "ECC_Pawn" "ECR_Block"))
    (:`then_1`
      (if (`self.Enabled`)
        (`ActorComponent.SetActive` (`self.StorageChassis`) false false)
        (`ClickableComponent.SetActiveUseContext` (`self.ClickableComponent`) "UC_TurnOff")))))

(event `self.StartInWorld`
  (goto _label))

(event `self.PlacedInSlot`
  (params (Slot :type "SlotReference Structure") (FromTool :type Boolean) (SlottedDuringInitialization :type Boolean))
  (goto _label))

(event `self.DroppedInWorld`
  (params (Component :type "PrimitiveComponent Object Reference") (NewTerrainComponent :type Boolean) (Point :type "Vector Structure (by ref)") (Normal :type "Vector Structure (by ref)"))
  (if NewTerrainComponent
    (`GameplayStatics.PlaySoundAtLocation` "/Game/Mods/TheCodingPro/BuildingBlocks/LockPlatform.LockPlatform" (`self.K2_GetActorLocation`) (struct) 1.0 1.0 0.0 null null null)))

(event `self.PickedUpFromWorld`
  (`GameplayStatics.PlaySoundAtLocation` "/Game/Mods/TheCodingPro/BuildingBlocks/UnlockPlatform.UnlockPlatform" (`self.K2_GetActorLocation`) (struct) 1.0 1.0 0.0 null null null))

(event `InputAction|Use`
  (params (Key :type "Key Structure"))
  (bind _storagechassis (`self.StorageChassis`))
  (bind _clickablecomponent (`self.ClickableComponent`))
  (:`Pressed`
    (if (`self.Enabled`)
      (`ActorComponent.SetActive` _storagechassis false false)
      (set `self.Enabled` true)
      (`ClickableComponent.SetActiveUseContext` _clickablecomponent "UC_TurnOff")
      (else
        (`ActorComponent.SetActive` _storagechassis true false)
        (set `self.Enabled` false)
        (`ClickableComponent.SetActiveUseContext` _clickablecomponent "UC_TurnOn")))))

(fn `GetBodySlotLegacy`
  (returns (ReturnValue :type "ChildSlotComponent Object Reference"))
  (return (`self.BodySlot`)))

(fn `UserConstructionScript`)