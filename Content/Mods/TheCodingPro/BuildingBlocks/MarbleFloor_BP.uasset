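; Marble floor building block, a slot-based placeable that keeps itself and any item on it solid to pawns.
; On begin play, world start or slot placement, it enables query and physics collision on its static mesh and blocks the Pawn channel.
; Every Tick reapplies that collision to the first TopSlot item's static mesh, falling back to its skeletal mesh.
; BottomSlot serves as its legacy body slot.
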(event `self.ReceiveBeginPlay`
  (bind _staticmeshcomponent (`self.StaticMeshComponent`))
  (`PrimitiveComponent.SetCollisionEnabled` _staticmeshcomponent "QueryAndPhysics" :!label _label)
  (`PrimitiveComponent.SetCollisionResponseToChannel` _staticmeshcomponent "ECC_Pawn" "ECR_Block"))

(event `self.StartInWorld`
  (goto _label))

(event `self.PlacedInSlot`
  (params (Slot :type "SlotReference Structure") (FromTool :type Boolean) (SlottedDuringInitialization :type Boolean))
  (goto _label))

(event `self.ReceiveTick`
  (params (DeltaSeconds :type "Float (single-precision)"))
  (bind _returnvalue (`SlotsComponent.GetSlotItem` (`ChildSlotComponent.MakeReference` (`self.TopSlot`))))
  (bind _returnvalue_2 (`self.GetComponentByClass` _returnvalue "/Script/Engine.SkeletalMeshComponent"))
  (bind _returnvalue_3 (`self.GetComponentByClass` _returnvalue "/Script/Engine.StaticMeshComponent"))
  (if (`KismetSystemLibrary.IsValid` _returnvalue)
    (if (`KismetSystemLibrary.IsValid` _returnvalue_3)
      (bind _output_get (set `self.StaticMeshRef` _returnvalue_3))
      (`PrimitiveComponent.SetCollisionEnabled` _output_get "QueryAndPhysics")
      (`PrimitiveComponent.SetCollisionResponseToChannel` _output_get "ECC_Pawn" "ECR_Block")
      (elif (`KismetSystemLibrary.IsValid` _returnvalue_2)
        (bind _output_get_2 (set `self.SkeletalMeshRef` _returnvalue_2))
        (`PrimitiveComponent.SetCollisionEnabled` _output_get_2 "QueryAndPhysics")
        (`PrimitiveComponent.SetCollisionResponseToChannel` _output_get_2 "ECC_Pawn" "ECR_Block")))))

(fn `GetBodySlotLegacy`
  (returns (ReturnValue :type "ChildSlotComponent Object Reference"))
  (return (`self.BottomSlot`)))

(fn `UserConstructionScript`)