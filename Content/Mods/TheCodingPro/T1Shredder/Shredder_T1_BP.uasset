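; T1 Shredder machine Blueprint from a mod, reskinning components inherited from its parent class.
; Every Tick assigns the T1Shredder skeletal mesh and collision static mesh to the first component of each type.
; It also moves the first ChildSlotComponent down along Z if its display name is BodySlot or InputSlot.
; Parent Tick runs only in the BodySlot branch, and the OutputSlot check is left unused.
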(event `self.ReceiveTick`
  (params (DeltaSeconds :type "Float (single-precision)"))
  (bind _returnvalue (`self.GetComponentByClass` self "/Script/Astro.ChildSlotComponent"))
  (bind _returnvalue_2 (`KismetSystemLibrary.GetDisplayName` _returnvalue))
  (`SkinnedMeshComponent.SetSkinnedAssetAndUpdate` (`self.GetComponentByClass` self "/Script/Engine.SkeletalMeshComponent") "/Game/Mods/TheCodingPro/T1Shredder/Models/T1Shredder.T1Shredder" false)
  (`StaticMeshComponent.SetStaticMesh` (`self.GetComponentByClass` self "/Script/Engine.StaticMeshComponent") "/Game/Mods/TheCodingPro/T1Shredder/Models/T1Shredder_Collision.T1Shredder_Collision")
  (`|ExecutionSequence`
    (:`then_0`
      (if (`KismetStringLibrary.EqualEqual_StrStr` _returnvalue_2 "BodySlot")
        (`SceneComponent.K2_SetRelativeLocation` _returnvalue (0.0 0.0 -90.0) false false)
        (`parent.ReceiveTick` DeltaSeconds)))
    (:`then_1`
      (if (`KismetStringLibrary.EqualEqual_StrStr` _returnvalue_2 "InputSlot")
        (`SceneComponent.K2_SetRelativeLocation` _returnvalue (0.0 0.0 -90.0) false false)))))

(fn `UserConstructionScript`
  (`parent.UserConstructionScript`))