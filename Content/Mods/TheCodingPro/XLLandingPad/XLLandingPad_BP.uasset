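; Deployable XL landing pad mod actor that the player locks in place or collapses with the Use action.
; Use flips IsMovable, deploys or tears down the LandingPad component, and switches the indicator light materials, lock sound and Deploy/Collapse prompt.
; Tick's terrain-attachment handling consists of disabled nodes.
; BeginPlay is empty, leaving the logic to restore a locked pad after reload unconnected.
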(event `InputAction|Use`
  (params (Key :type "Key Structure"))
  (bind _clickablecomponent (`self.ClickableComponent`))
  (bind _landingpad (`self.LandingPad`))
  (bind _lightindicator1 (`self.LightIndicator1`))
  (bind _lightindicator2 (`self.LightIndicator2`))
  (:`Pressed`
    (if (`self.IsMovable`)
      ;[1 1 1] Sets IsMovable to true or false
      (set `self.IsMovable` false)
      ;[1 1 1] Deploys or Tearsdown the Landing Pad
      (`LandingPadComponent.AuthorityDeployLandingPad` _landingpad)
      ;[1 1 1] Set the Indicator Light's material to glow or not
      (`PrimitiveComponent.SetMaterial` _lightindicator1 1 "/Game/Mods/TheCodingPro/XLLandingPad/Pole_Light_Enabled.Pole_Light_Enabled")
      (`PrimitiveComponent.SetMaterial` _lightindicator2 1 "/Game/Mods/TheCodingPro/XLLandingPad/Pole_Light_Enabled.Pole_Light_Enabled")
      ;[1 1 1] Plays locking or unlocking sound
      (`AstroStatics.PlaySound` "/Game/Mods/TheCodingPro/XLLandingPad/LockPlatform.LockPlatform")
      ;[1 1 1] The SetActiveUseContext method allows you to change what displays as the use action and automatically refreshes active tooltips if necessary
      (`ClickableComponent.SetActiveUseContext` _clickablecomponent "UC_Collapse")
      (else
        (set `self.IsMovable` true)
        (`LandingPadComponent.AuthorityTeardownLandingPad` _landingpad)
        (`PrimitiveComponent.SetMaterial` _lightindicator1 1 "/Game/Mods/TheCodingPro/XLLandingPad/Pole_Light_Disabled.Pole_Light_Disabled")
        (`PrimitiveComponent.SetMaterial` _lightindicator2 1 "/Game/Mods/TheCodingPro/XLLandingPad/Pole_Light_Disabled.Pole_Light_Disabled")
        (`AstroStatics.PlaySound` "/Game/Mods/TheCodingPro/XLLandingPad/UnlockPlatform.UnlockPlatform")
        (`ClickableComponent.SetActiveUseContext` _clickablecomponent "UC_Deploy")))))

(event `self.ReceiveBeginPlay`
  ;[1 1 1] Keeps platform locked between reloading save and sets some stuff up
)

(event `self.ReceiveTick`
  (params (DeltaSeconds :type "Float (single-precision)"))
  (bind _clickablecomponent (`self.ClickableComponent`))
  ;[1 1 1] Checks every tick on whether the landing pad is attached to the terrain
  (if (`self.bIsAttachedToTerrain`)
    (set `ClickableComponent.UseSuppressionState` (make `UseSuppressionState` "None" :!enabledstate Disabled) _clickablecomponent :!enabledstate Disabled)
    (else
      (set `ClickableComponent.UseSuppressionState` (make `UseSuppressionState` "All" :!enabledstate Disabled) _clickablecomponent :!enabledstate Disabled)
      (`LandingPadComponent.AuthorityTeardownLandingPad` (`self.LandingPad` :!enabledstate Disabled) :!enabledstate Disabled)
      (set `self.IsMovable` true :!enabledstate Disabled))))

(fn `GetBodySlotLegacy`
  (returns (ReturnValue :type "ChildSlotComponent Object Reference"))
  (return (`self.BodySlot`)))

(fn `UserConstructionScript`)